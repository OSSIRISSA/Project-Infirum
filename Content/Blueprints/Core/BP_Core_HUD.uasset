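; BP_Core_HUD is the HUD Blueprint that sets up the in-game screen for the owning player.
; On BeginPlay it switches input to game-only, then creates WBP_MainGUI, stores it and adds it to the viewport.
; It then hands the GUI's PlayerInventory widget to the Cryptor on BP_Core_PC as its WidgetRef, linking the inventory UI to the player controller.
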(event `self.ReceiveBeginPlay`
  (`WidgetBlueprintLibrary.SetInputMode_GameOnly` (`self.GetOwningPlayerController`))
  ;[1 1 1] IngameScreen
  (bind _returnvalue (`|CreateWidget` "/Game/GUI/WBP_MainGUI.WBP_MainGUI_C" (`self.GetOwningPlayerController`)))
  (bind _output_get (set `self.MainGUI` _returnvalue))
  (`UserWidget.AddToViewport` _output_get 0)
  ;[1 1 1] Inventories
  (set `/Game/Blueprints/Inventory/BP_MainCryptor.WidgetRef` (`/Game/GUI/WBP_MainGUI.PlayerInventory` (`self.MainGUI`)) (`/Game/Blueprints/Core/BP_Core_PC.Cryptor` (cast `/Game/Blueprints/Core/BP_Core_PC` (`self.GetOwningPlayerController`) :!pure true))))

(fn `UserConstructionScript`)