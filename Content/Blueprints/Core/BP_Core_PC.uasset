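; Player controller that handles inventory and container UI modes and forwards mouse input to the player's widget interaction component.
; ChangeControlMode tracks player and container open states by cryptor type, sets parent widget visibility and calls ToShowMouseCursor to switch cursor and input mode.
; The inventory action toggles the player's inventory widget component and interaction distance.
; Left clicks also pass the player reference to hovered widgets, and a temporary Tick print shows state flags.
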(event `InputAxisKey|MouseWheelAxis`
  (params (AxisValue :type "Float (single-precision)"))
  ; Widget Interaction
  (`WidgetInteractionComponent.ScrollWheel` (`/Game/Blueprints/BP_Player.WidgetInteraction` (`self.PlayerRef`)) AxisValue))

(event `Key|RightMouseButton`
  (params (Key :type "Key Structure"))
  (bind _widgetinteraction (`/Game/Blueprints/BP_Player.WidgetInteraction` (`self.PlayerRef`)))
  ; Widget Interaction
  (:`Pressed`
    (`WidgetInteractionComponent.PressPointerKey` _widgetinteraction Key))
  (:`Released`
    (`WidgetInteractionComponent.ReleasePointerKey` _widgetinteraction Key)))

(event `Key|LeftMouseButton`
  (params (Key :type "Key Structure"))
  (bind _widgetinteraction (`/Game/Blueprints/BP_Player.WidgetInteraction` (`self.PlayerRef`)))
  (bind _returnvalue (`WidgetInteractionComponent.GetHoveredWidgetComponent` _widgetinteraction))
  ; Widget Interaction
  (:`Pressed`
    (`WidgetInteractionComponent.PressPointerKey` _widgetinteraction Key)
    (`/Engine/EditorBlueprintResources/StandardMacros.IsValid` _returnvalue
      (:`Is Valid`
        (message `/Game/Blueprints/BPI_SetPlayerRef.SetPlayerRef` (`WidgetComponent.GetWidget` _returnvalue) (`self.PlayerRef`)))))
  (:`Released`
    (`WidgetInteractionComponent.ReleasePointerKey` _widgetinteraction Key)))

(event `EnhancedInput|/Game/Blueprints/Input/IA_OpenInventory`
  (params (ActionValue :type Boolean) (ElapsedSeconds :type "Float (double-precision)") (TriggeredSeconds :type "Float (double-precision)") (InputAction :type "InputAction Object Reference" :default "/Game/Blueprints/Input/IA_OpenInventory.IA_OpenInventory"))
  (bind _inventorywidgetcomponent (`/Game/Blueprints/BP_Player.InventoryWidgetComponent` (`self.PlayerRef`)))
  (bind _widgetinteraction (`/Game/Blueprints/BP_Player.WidgetInteraction` (`self.PlayerRef`)))
  ;[0 0 1 0.4] Open/Close Inventory
  (:`Triggered`
    (if (`self.bInventoryOpened`)
      (`self.changeControlMode` "NewEnumerator0" null (`/Game/Blueprints/BP_Player.InventoryWidget` (`self.PlayerRef`)))
      (`SceneComponent.SetVisibility` _inventorywidgetcomponent false false)
      (if (not (`self.bShowMouseCursor`))
        (set `WidgetInteractionComponent.InteractionDistance` 0.0 _widgetinteraction))
      (else
        (`self.changeControlMode` "NewEnumerator1" null (`/Game/Blueprints/BP_Player.InventoryWidget` (`self.PlayerRef`)))
        (`SceneComponent.SetVisibility` _inventorywidgetcomponent true false)
        (set `WidgetInteractionComponent.InteractionDistance` 500.0 _widgetinteraction)))))

(event `self.ReceiveTick`
  (params (DeltaSeconds :type "Float (single-precision)"))
  ;[0 1 0 0.5] TEMP
  (`KismetSystemLibrary.PrintString` (`KismetStringLibrary.Concat_StrStr` "Inventory Opened: " (`KismetStringLibrary.Conv_BoolToString` (`self.bInventoryOpened`)) " \nContainer Opened: " (`KismetStringLibrary.Conv_BoolToString` (`self.bContainerOpened`)) " \nIs Splitting:             " (`KismetStringLibrary.Conv_BoolToString` (`self.bIsSplitting`))) true true (struct :`R` 0.099325 :`G` 0.274306 :`B` 0.097332 :`A` 1.0) 0.0))

(event `SetPlayerRef`
  (params (Player :type "/Game/Blueprints/BP_Player Object Reference"))
  ;[0.7344 0.3894 0 0.5] Set Player
  (set `self.PlayerRef` Player))

(event `self.ReceiveBeginPlay`
  ;[1 0 0 0.3] BeginPlay
  (set `self.HUD` (cast `/Game/Blueprints/Core/BP_Core_HUD` (`self.GetHUD`) :!pure true)))

(fn `changeControlMode`
  (params (`New Control` :type "/Game/Blueprints/Core/E_ControlType Enum" :default "NewEnumerator0") (CryptorParent :type "/Game/GUI/WBP_MovableTitleBar Object Reference") (CryptorWBP :type "/Game/GUI/WBP_MainCryptor Object Reference"))
  (switch `/Game/Blueprints/Core/E_ControlType` `New Control`
    (:`NewEnumerator0`
      (switch `/Game/Blueprints/Inventory/E_CryptorType` (`/Game/GUI/WBP_MainCryptor.CryptorType` (`local.CryptorWBP`))
        (:`NewEnumerator0`
          (if (`self.bInventoryOpened`)
            (set `self.bInventoryOpened` false)
            (bind _cryptorparent (`local.CryptorParent` :!label _label)
              (:`then`
                (`Widget.SetVisibility` _cryptorparent "Collapsed"))
              (:`else`
                _))
            (`self.toShowMouseCursor` null)
            (if (`KismetMathLibrary.BooleanNOR` (`self.bInventoryOpened`) (`self.bContainerOpened`))
              (set `self.CurrentControlMode` "NewEnumerator0"))))
        (:`NewEnumerator1`
          (if (`self.bContainerOpened`)
            (set `self.bContainerOpened` false)
            (goto _label)))))
    (:`NewEnumerator1`
      (switch `/Game/Blueprints/Inventory/E_CryptorType` (`/Game/GUI/WBP_MainCryptor.CryptorType` (`local.CryptorWBP`))
        (:`NewEnumerator0`
          (set `self.bInventoryOpened` true))
        (:`NewEnumerator1`
          (set `self.bContainerOpened` true)))
      (bind _cryptorparent_2 (`local.CryptorParent`)
        (:`then`
          (`Widget.SetVisibility` _cryptorparent_2 "Visible")
          (`self.toShowMouseCursor` (`local.CryptorParent`)))
        (:`else`
          (`self.toShowMouseCursor` null)))
      (set `self.CurrentControlMode` "NewEnumerator1"))))

(fn `toShowMouseCursor`
  (params (InWidgetToFocus :type "Widget Object Reference"))
  (bind _output_get (set `self.bShowMouseCursor` (or (`self.bInventoryOpened`) (`self.bContainerOpened`) (`self.bIsSplitting`))))
  (if _output_get
    (`/Engine/EditorBlueprintResources/StandardMacros.IsValid` InWidgetToFocus
      (:`Is Valid`
        (`WidgetBlueprintLibrary.SetInputMode_GameAndUIEx` self InWidgetToFocus "DoNotLock" false))
      (:`Is Not Valid`
        (`WidgetBlueprintLibrary.SetInputMode_GameAndUIEx` self null "DoNotLock" false)))
    (else
      (`WidgetBlueprintLibrary.SetInputMode_GameOnly` self))))

(fn `UserConstructionScript`)