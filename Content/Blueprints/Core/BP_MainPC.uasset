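; Main player controller that owns the in-game screen widget and handles opening and closing the inventory.
; On BeginPlay it caches the player pawn, adds the screen to the viewport and builds its inventory from Cryptor.
; The inventory input action toggles widget visibility, input mode, mouse cursor and an opened flag together.
; Tick prints each Cryptor item's class and quantity on screen every frame as debug output.
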(event `self.ReceiveBeginPlay`
  (set `self.PlayerRef` (cast `/Game/Blueprints/BP_Player` (`self.K2_GetPawn`) :!pure true))
  (bind _returnvalue (`|CreateWidget` "/Game/GUI/WBP_InGameScreen.WBP_InGameScreen_C" self self))
  (bind _output_get (set `self.InGameScreen` _returnvalue))
  (`UserWidget.AddToViewport` _output_get 0)
  (`/Game/GUI/WBP_InGameScreen.CreateInventory` (`self.InGameScreen`) (`self.Cryptor`)))

(event `EnhancedInput|/Game/Blueprints/Input/Actions/IA_OpenInventory`
  (params (ActionValue :type Boolean) (ElapsedSeconds :type "Float (double-precision)") (TriggeredSeconds :type "Float (double-precision)") (InputAction :type "InputAction Object Reference" :default "/Game/Blueprints/Input/Actions/IA_OpenInventory.IA_OpenInventory"))
  ;[0 0 1 0.4] Open/Close Inventory
  (:`Triggered`
    (switch `ESlateVisibility` (`Widget.GetVisibility` (`/Game/GUI/WBP_InGameScreen.Inventory` (`self.InGameScreen`)))
      (:`Visible`
        (`Widget.SetVisibility` (`/Game/GUI/WBP_InGameScreen.Inventory` (`self.InGameScreen`)) "Hidden")
        (`WidgetBlueprintLibrary.SetInputMode_GameOnly` self)
        (set `self.bShowMouseCursor` false)
        (set `self.InventoryOpened` false))
      (:`Hidden`
        (`Widget.SetVisibility` (`/Game/GUI/WBP_InGameScreen.Inventory` (`self.InGameScreen`)) "Visible")
        (`WidgetBlueprintLibrary.SetInputMode_GameAndUIEx` self (`/Game/GUI/WBP_InGameScreen.Inventory` (`self.InGameScreen`)))
        (set `self.bShowMouseCursor` true)
        (set `self.InventoryOpened` true)))))

(event `self.ReceiveTick`
  (params (DeltaSeconds :type "Float (single-precision)"))
  (bind _values (`BlueprintMapLibrary.Map_Values` (`/Game/Blueprints/Inventory/BP_MainCryptor.Items` (`self.Cryptor`))))
  (for _array_element _values
    (`KismetSystemLibrary.PrintString` (`KismetStringLibrary.Concat_StrStr` (`KismetSystemLibrary.GetClassDisplayName` (break `/Game/Blueprints/Items/S_ItemInventoryUnique` _array_element)) " -- " (`KismetStringLibrary.Conv_IntToString` (`.Quantity_9_DC4C08534AC362A1F305B0BE75112C5F` (break `/Game/Blueprints/Items/S_ItemInventoryUnique` _array_element)))) true true (struct :`G` 0.66 :`B` 1.0 :`A` 1.0) 0.0)))

(fn `UserConstructionScript`)