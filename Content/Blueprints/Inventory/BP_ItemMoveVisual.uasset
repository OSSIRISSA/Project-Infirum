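; World-space widget component on BP_Player that displays an inventory item under the mouse cursor, apparently while it is being moved.
; ShowItemVisual fills the WBP_ItemSlot widget and enables visibility and ticking; HideItemVisual disables both.
; Tick traces from the deprojected cursor, placing the widget short of any hit or at maximum range, turned toward the first-person camera.
; Scale follows distance only on hits, and debug drawing and prints remain active.
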(event `self.ReceiveTick`
  (params (DeltaSeconds :type "Float (single-precision)"))
  (bind (_returnvalue_roll _returnvalue_pitch _returnvalue_yaw) (`KismetMathLibrary.BreakRotator` (`self.K2_GetComponentRotation`)))
  (bind _returnvalue_roll_2 (`KismetMathLibrary.BreakRotator` (`self.K2_GetComponentRotation`)))
  (bind _asbp_player (cast `/Game/Blueprints/BP_Player` (`self.GetOwner`) :!pure true))
  (bind (_worldlocation _worlddirection) (`PlayerController.DeprojectMousePositionToWorld` (`/Game/Blueprints/BP_Player.PlayerController` _asbp_player)))
  (bind (_returnvalue_roll_3 _returnvalue_pitch_2 _returnvalue_yaw_2) (`KismetMathLibrary.BreakRotator` (`KismetMathLibrary.FindLookAtRotation` (`self.K2_GetComponentLocation` (`/Game/Blueprints/BP_Player.FirstPersonCamera` _asbp_player)) (`self.K2_GetComponentLocation`))))
  (bind _returnvalue (+ _worldlocation (* _worlddirection 500.0)))
  (bind _returnvalue_2 (`KismetMathLibrary.MakeRotator` _returnvalue_roll_2 (* _returnvalue_pitch_2 -1.0) (+ _returnvalue_yaw_2 180.0)))
  (bind (_outhit _returnvalue_3) (`KismetSystemLibrary.LineTraceSingle` :`Start` _worldlocation :`End` _returnvalue :`TraceChannel` "TraceTypeQuery1" :`DrawDebugType` "ForOneFrame"))
  (if _returnvalue_3
    (bind (_bblockinghit _binitialoverlap _time _distance _location _impactpoint _normal _impactnormal _physmat _hitactor _hitcomponent _hitbonename _bonename _hititem _elementindex _faceindex _tracestart _traceend) (`GameplayStatics.BreakHitResult` _outhit))
    (bind _returnvalue_4 (`KismetMathLibrary.ClampVectorSize` (* (- _location _tracestart) 0.8) 0.0 500.0))
    (`self.K2_SetWorldLocation` (+ _returnvalue_4 _tracestart) false true)
    (`self.K2_SetWorldRotation` _returnvalue_2)
    ; Prints
    (`KismetSystemLibrary.PrintString` (`KismetStringLibrary.Concat_StrStr` "X " (`KismetStringLibrary.Conv_DoubleToString` _returnvalue_roll) " \nY " (`KismetStringLibrary.Conv_DoubleToString` _returnvalue_pitch) " \nZ " (`KismetStringLibrary.Conv_DoubleToString` _returnvalue_yaw)) true false (struct :`G` 0.66 :`B` 1.0 :`A` 1.0) 0.0)
    (bind _returnvalue_5 (+ (`KismetMathLibrary.NormalizeToRange` (/ (`KismetMathLibrary.VSize` _returnvalue_4) 500.0) 0.0 5.0) 0.025))
    (`self.SetWorldScale3D` (`KismetMathLibrary.MakeVector` _returnvalue_5 _returnvalue_5 _returnvalue_5))
    (else
      (`KismetSystemLibrary.PrintString` (`KismetStringLibrary.Concat_StrStr` (`KismetStringLibrary.Conv_VectorToString` _worldlocation) " \n" (`KismetStringLibrary.Conv_VectorToString` _worlddirection)) true true (struct :`R` 1.0 :`G` 0.267512 :`A` 1.0) 0.0)
      (`self.K2_SetWorldLocation` _returnvalue false true)
      (`self.K2_SetWorldRotation` _returnvalue_2))))

(fn `HideItemVisual`
  (`self.SetVisibility` false)
  (`self.SetTickMode` "Disabled"))

(fn `ShowItemVisual`
  (params (Item :type "/Game/GUI/WBP_ItemSlot Object Reference"))
  (bind _item (`local.Item`))
  (`/Game/GUI/WBP_ItemSlot.updateSlotStatus` (cast `/Game/GUI/WBP_ItemSlot` (`self.GetWidget`) :!pure true) (`/Game/GUI/WBP_ItemSlot.Item` _item) (`/Game/GUI/WBP_ItemSlot.Quantity` _item) (`/Game/GUI/WBP_ItemSlot.Durability` _item))
  (`self.SetVisibility` true)
  (`self.SetTickMode` "Enabled"))