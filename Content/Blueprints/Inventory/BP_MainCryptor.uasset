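; BP_MainCryptor is an inventory container holding a map from slot widgets to item class, quantity and durability.
; Adding tops up a stack with room or requests a new slot from the widget; splitting opens the HUD's splitter.
; Swaps work across containers through each slot's cryptor reference, choosing between exchange, move, merge or overflow stacking.
; Removal cancels any active placement and spawns a drop-overlap actor attached to the player's camera.
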(fn `addItem`
  (params (ItemToAdd :type "/Game/Blueprints/Items/BP_MainItem Class Reference") (Count :type Integer) (Durability :type "Float (double-precision)"))
  (locals (lFoundItem :type "/Game/Blueprints/Items/S_ItemInventoryUnique Structure"))
  (bind (_lfounditem_itemclass _lfounditem_quantity) (break `/Game/Blueprints/Items/S_ItemInventoryUnique` (`local.lFoundItem`)))
  (bind (_lfounditem_itemclass_2 _lfounditem_quantity_2 _lfounditem_durability) (break `/Game/Blueprints/Items/S_ItemInventoryUnique` (`local.lFoundItem`)))
  (bind (_isrecyclable _iscraftable _itemname _weight _value _count _rarity _durability _equipability _isbreakablebytime _mesh _texture _stacksize) (defaults `Object` _lfounditem_itemclass))
  (bind _returnvalue (+ (`local.Count`) _lfounditem_quantity_2))
  (bind _keys (`BlueprintMapLibrary.Map_Keys` (`self.Items`)))
  (for _array_element _keys
    (set `local.lFoundItem` (`BlueprintMapLibrary.Map_Find` (`self.Items`) _array_element))
    (if (and (== _lfounditem_itemclass (`local.ItemToAdd`)) (or (>= (- _stacksize _lfounditem_quantity) (`local.Count`)) (<= _stacksize 0)) (not (`/Game/GUI/WBP_ItemSlot.bIsDragging` _array_element)))
      (`BlueprintMapLibrary.Map_Add` (`self.Items`) _array_element (make `/Game/Blueprints/Items/S_ItemInventoryUnique` _lfounditem_itemclass_2 _returnvalue _lfounditem_durability))
      (`/Game/GUI/WBP_ItemSlot.updateSlotStatus` _array_element _returnvalue _lfounditem_durability)
      (return)))
  ;[1 1 1] Taken Slot Was not Found, Adding New
  (bind _slotref (`/Game/GUI/WBP_MainCryptor.widgetAddNewItem` (`self.WidgetRef`) (`local.ItemToAdd`) (`local.Count`) (`local.Durability`)))
  (`BlueprintMapLibrary.Map_Add` (`self.Items`) _slotref (make `/Game/Blueprints/Items/S_ItemInventoryUnique` (`local.ItemToAdd`) (`local.Count`) (`local.Durability`)))
  (`/Game/GUI/WBP_MainCryptor.checkForNewRow` (`self.WidgetRef`))
  (return))

(fn `InvalidateSlot`
  (params (Slot :type "/Game/GUI/WBP_ItemSlot Object Reference"))
  (`BlueprintMapLibrary.Map_Remove` (`/Game/Blueprints/Inventory/BP_MainCryptor.Items` (`/Game/GUI/WBP_ItemSlot.CryptorRef` Slot)) Slot))

(fn `removeItem`
  (params (PlayerController :type "PlayerController Object Reference") (itemToRemove :type "/Game/GUI/WBP_ItemSlot Object Reference") (ItemToSpawn :type "/Game/Blueprints/Items/S_ItemInventoryUnique Structure"))
  (locals (lPlayerController :type "/Game/Blueprints/Core/BP_Core_PC Object Reference"))
  (bind _playerref (`/Game/Blueprints/Core/BP_Core_PC.PlayerRef` (`local.lPlayerController`)))
  (bind _followcamera (`/Game/Blueprints/BP_Player.FollowCamera` (`/Game/Blueprints/Core/BP_Core_PC.PlayerRef` (`local.lPlayerController`))))
  (set `local.lPlayerController` (cast `/Game/Blueprints/Core/BP_Core_PC` PlayerController :!pure true))
  (`/Game/Blueprints/BP_Player.PlaceableItem` _playerref
    (:`then`
      (`/Game/Blueprints/BP_Player.CancelPlacingItem` _playerref))
    (:`else`
      _))
  (`/Game/GUI/WBP_ItemSlot.invalidateSlot` (`local.itemToRemove`))
  (bind _returnvalue (`|SpawnActorFromClass` "/Game/Blueprints/Items/BP_ItemDrawOverlap.BP_ItemDrawOverlap_C" (`KismetMathLibrary.MakeTransform` (+ (`SceneComponent.K2_GetComponentLocation` _followcamera) (* (`SceneComponent.GetForwardVector` _followcamera) (`self.ItemDropDistance`)))) "AlwaysSpawn" "MultiplyWithRoot" (`local.lPlayerController`) (`local.ItemToSpawn`) self null))
  (`Actor.K2_AttachToComponent` _returnvalue (`/Game/Blueprints/BP_Player.FollowCamera` (`/Game/Blueprints/Core/BP_Core_PC.PlayerRef` (`local.lPlayerController`))) "None" "KeepWorld" "KeepRelative" "KeepWorld" false)
  (`BlueprintMapLibrary.Map_Remove` (`self.Items`) (`local.itemToRemove`)))

(fn `SetSlot`
  (params (Slot :type "/Game/GUI/WBP_ItemSlot Object Reference") (Item :type "/Game/Blueprints/Items/S_ItemInventoryUnique Structure"))
  (bind (_item_itemclass _item_quantity _item_durability) (break `/Game/Blueprints/Items/S_ItemInventoryUnique` (`local.Item`)))
  (`BlueprintMapLibrary.Map_Add` (`/Game/Blueprints/Inventory/BP_MainCryptor.Items` (`/Game/GUI/WBP_ItemSlot.CryptorRef` (`local.Slot`))) Slot Item)
  (set `/Game/GUI/WBP_ItemSlot.Item` _item_itemclass (`local.Slot`))
  (`/Game/GUI/WBP_ItemSlot.updateSlotStatus` (`local.Slot`) _item_quantity _item_durability))

(fn `splitItem`
  (params (itemToRemove :type "/Game/GUI/WBP_ItemSlot Object Reference"))
  (locals (lPlayerController :type "/Game/Blueprints/Core/BP_Core_PC Object Reference"))
  (bind _output_get (set `local.lPlayerController` (cast `/Game/Blueprints/Core/BP_Core_PC` (`GameplayStatics.GetPlayerController` 0) :!pure true)))
  (set `/Game/Blueprints/Core/BP_Core_PC.bIsSplitting` true _output_get)
  (`/Game/GUI/WBP_SplitItems.ToShowSplitter` (`/Game/GUI/WBP_MainGUI.ItemsSplitter` (`/Game/Blueprints/Core/BP_Core_HUD.MainGUI` (cast `/Game/Blueprints/Core/BP_Core_HUD` (`PlayerController.GetHUD` (`local.lPlayerController`)) :!pure true))) (`BlueprintMapLibrary.Map_Find` (`self.Items`) (`local.itemToRemove`)) (`local.itemToRemove`)))

(fn `swapItems`
  (params (PrimarySlot :type "/Game/GUI/WBP_ItemSlot Object Reference") (SecondarySlot :type "/Game/GUI/WBP_ItemSlot Object Reference"))
  (locals (FirstStruct :type "/Game/Blueprints/Items/S_ItemInventoryUnique Structure") (SecondStruct :type "/Game/Blueprints/Items/S_ItemInventoryUnique Structure"))
  (bind (_firststruct_itemclass _firststruct_quantity _firststruct_durability) (break `/Game/Blueprints/Items/S_ItemInventoryUnique` (`local.FirstStruct`)))
  (bind (_secondstruct_itemclass _secondstruct_quantity _secondstruct_durability) (break `/Game/Blueprints/Items/S_ItemInventoryUnique` (`local.SecondStruct`)))
  (bind (_firststruct_itemclass_2 _firststruct_quantity_2 _firststruct_durability_2) (break `/Game/Blueprints/Items/S_ItemInventoryUnique` (`local.FirstStruct`)))
  (bind (_isrecyclable _iscraftable _itemname _weight _value _count _rarity _durability _equipability _isbreakablebytime _mesh _texture _stacksize) (defaults `Object` _secondstruct_itemclass))
  (set `local.FirstStruct` (`BlueprintMapLibrary.Map_Find` (`/Game/Blueprints/Inventory/BP_MainCryptor.Items` (`/Game/GUI/WBP_ItemSlot.CryptorRef` (`local.PrimarySlot`))) (`local.PrimarySlot`)))
  (set `local.SecondStruct` (`BlueprintMapLibrary.Map_Find` (`self.Items`) (`local.SecondarySlot`)))
  (bind _addamount (`self.SwitchWayOfSwap` (`local.FirstStruct`) (`local.SecondStruct`))
    (:`DefaultSwap`
      (`self.SetSlot` (`local.PrimarySlot`) (`local.SecondStruct`))
      (`self.SetSlot` (`local.SecondarySlot`) (`local.FirstStruct`) :!label _label))
    (:`MoveItem`
      (`/Game/GUI/WBP_ItemSlot.invalidateSlot` (`local.PrimarySlot`))
      (`self.InvalidateSlot` (`local.PrimarySlot`))
      (goto _label))
    (:`PerfectStackItem`
      (`/Game/GUI/WBP_ItemSlot.invalidateSlot` (`local.PrimarySlot`))
      (`self.InvalidateSlot` (`local.PrimarySlot`))
      (`self.SetSlot` (`local.SecondarySlot`) (make `/Game/Blueprints/Items/S_ItemInventoryUnique` _firststruct_itemclass_2 _addamount _firststruct_durability_2)))
    (:`OverStackItems`
      (`self.SetSlot` (`local.PrimarySlot`) (make `/Game/Blueprints/Items/S_ItemInventoryUnique` _firststruct_itemclass (- (+ _firststruct_quantity _secondstruct_quantity) _stacksize) _firststruct_durability))
      (`self.SetSlot` (`local.SecondarySlot`) (make `/Game/Blueprints/Items/S_ItemInventoryUnique` _secondstruct_itemclass _stacksize _secondstruct_durability))))
  (`/Game/GUI/WBP_MainCryptor.checkForNewRow` (`self.WidgetRef`)))