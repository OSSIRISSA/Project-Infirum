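; BP_MainContainer is an interactable container actor that shows its items in a grid inventory widget.
; The first interaction begin creates a WBP_MainCryptor from Columns, Rows and Items and assigns it to the widget component, while every begin enables custom depth on the mesh.
; The action toggles the widget and player control mode based on the controller's ContainerOpened.
; Ending interaction clears custom depth and, if the widget exists, hides it and switches control mode.
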(event `/Game/Blueprints/Inventory/IBP_Interactable.OnInteractionAction`
  (params (PlayerController :type "/Game/Blueprints/Core/BP_Core_PC Object Reference"))
  ; Action Interaction
  (if (`/Game/Blueprints/Core/BP_Core_PC.bContainerOpened` PlayerController)
    (`/Game/Blueprints/Core/BP_Core_PC.changeControlMode` PlayerController "NewEnumerator0" null (`self.InventoryWidget`))
    (`SceneComponent.SetVisibility` (`self.InventoryWidgetComponent`) false false)
    (else
      (`/Game/Blueprints/Core/BP_Core_PC.changeControlMode` PlayerController "NewEnumerator1" null (`self.InventoryWidget`))
      (`SceneComponent.SetVisibility` (`self.InventoryWidgetComponent`) true false))))

(event `/Game/Blueprints/Inventory/IBP_Interactable.OnInteractionend`
  (params (PlayerController :type "/Game/Blueprints/Core/BP_Core_PC Object Reference"))
  ; End Interaction
  (`PrimitiveComponent.SetRenderCustomDepth` (`self.Mesh`) false)
  (bind _inventorywidget (`self.InventoryWidget`)
    (:`then`
      (`/Game/Blueprints/Core/BP_Core_PC.changeControlMode` PlayerController "NewEnumerator0" null _inventorywidget)
      (`SceneComponent.SetVisibility` (`self.InventoryWidgetComponent`) false false))
    (:`else`)))

(event `/Game/Blueprints/Inventory/IBP_Interactable.OnInteractionBegin`
  ; Begin Interaction
  (`|ExecutionSequence`
    (:`then_0`
      (`/Engine/EditorBlueprintResources/StandardMacros.DoOnce` false
        (:`Completed`
          (bind _returnvalue (`|CreateWidget` "/Game/GUI/WBP_MainCryptor.WBP_MainCryptor_C" null (`self.Columns`) (`self.Rows`) "NewEnumerator1" false true null))
          (bind _output_get (set `self.InventoryWidget` _returnvalue))
          (`WidgetComponent.SetWidget` (`self.InventoryWidgetComponent`) _output_get)
          (`/Game/GUI/WBP_MainCryptor.updateInventory` (`self.InventoryWidget`) (`self.Items`)))))
    (:`then_1`
      (`PrimitiveComponent.SetRenderCustomDepth` (`self.Mesh`) true))))

(fn `IsInteractable`
  (returns (isInteractable :type Boolean))
  (return true))

(fn `UserConstructionScript`)