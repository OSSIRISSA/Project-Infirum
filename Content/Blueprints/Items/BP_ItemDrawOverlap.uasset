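; Placement preview actor that shows a ghost of an item and follows the mouse cursor while the player chooses where to drop it.
; Construction copies the item class's mesh, tints it green and registers itself as the player's PlaceableItem.
; Each Tick traces from the deprojected cursor up to the drop distance, stopping just short of hits.
; Mesh overlaps toggle CanBePlaced and swap materials between red and green.
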(event `self.ItemMesh.OnComponentBeginOverlap`
  (params (OverlappedComponent :type "PrimitiveComponent Object Reference") (OtherActor :type "Actor Object Reference") (OtherComp :type "PrimitiveComponent Object Reference") (OtherBodyIndex :type Integer) (bFromSweep :type Boolean) (SweepResult :type "HitResult Structure (by ref)"))
  (set `self.bCanBePlaced` false)
  (for (_ _array_index) (`MeshComponent.GetMaterials` (`self.ItemMesh`))
    (`PrimitiveComponent.SetMaterial` (`self.ItemMesh`) _array_index "/Game/Blueprints/Items/M_Red.M_Red")))

(event `self.ItemMesh.OnComponentEndOverlap`
  (params (OverlappedComponent :type "PrimitiveComponent Object Reference") (OtherActor :type "Actor Object Reference") (OtherComp :type "PrimitiveComponent Object Reference") (OtherBodyIndex :type Integer))
  (set `self.bCanBePlaced` true)
  (for (_ _array_index) (`MeshComponent.GetMaterials` (`self.ItemMesh`))
    (`PrimitiveComponent.SetMaterial` (`self.ItemMesh`) _array_index "/Game/Blueprints/Items/M_Green.M_Green")))

(event `self.ReceiveTick`
  (params (DeltaSeconds :type "Float (single-precision)"))
  (bind (_worldlocation _worlddirection) (`PlayerController.DeprojectMousePositionToWorld` (`/Game/Blueprints/BP_Player.PlayerController` (`self.Player`))))
  (bind _returnvalue (+ _worldlocation (* _worlddirection (`/Game/Blueprints/BP_Player.CurrentDropDistance` (`self.Player`)))))
  (bind (_outhit _returnvalue_2) (`KismetSystemLibrary.LineTraceSingle` :`Start` _worldlocation :`End` _returnvalue :`TraceChannel` "TraceTypeQuery1" :`DrawDebugType` "ForOneFrame"))
  (if _returnvalue_2
    (bind (_bblockinghit _binitialoverlap _time _distance _location _impactpoint _normal _impactnormal _physmat _hitactor _hitcomponent _hitbonename _bonename _hititem _elementindex _faceindex _tracestart) (`GameplayStatics.BreakHitResult` _outhit))
    (`self.K2_SetActorLocation` (+ (`KismetMathLibrary.ClampVectorSize` (* (- _location _tracestart) 0.95) 0.0 500.0) _tracestart))
    (else
      (`self.K2_SetActorLocation` _returnvalue))))

(fn `UserConstructionScript`
  (bind _itemtospawn_itemclass (break `/Game/Blueprints/Items/S_Item` (`self.ItemToSpawn`)))
  (`StaticMeshComponent.SetStaticMesh` (`self.ItemMesh`) (defaults `Object` _itemtospawn_itemclass))
  (for (_ _array_index) (`MeshComponent.GetMaterials` (`self.ItemMesh`))
    (`PrimitiveComponent.SetMaterial` (`self.ItemMesh`) _array_index "/Game/Blueprints/Items/M_Green.M_Green"))
  (`self.K2_AddActorWorldOffset` (`KismetMathLibrary.MakeVector` 0.0 0.0 (* (.z (`.BoxExtent` (`KismetSystemLibrary.GetComponentBounds` (`self.ItemMesh`)))) -1.0)))
  (set `/Game/Blueprints/BP_Player.CurrentDropDistance` 300.0 (`self.Player`))
  (bind _placeableitem (`/Game/Blueprints/BP_Player.PlaceableItem` (`self.Player`))
    (:`then`
      (`KismetSystemLibrary.PrintString` "WTF. HOW IS IT VALID?"))
    (:`else`
      (`|VariableSetRef` _placeableitem self))))