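; BP_MainItem is a world item that the player picks up by walking into it.
; When BP_Player overlaps its Sphere, it passes its own class and Count to AddItem on the player controller's Cryptor, then destroys itself.
; The Construction Script applies the Mesh variable to the static mesh component, and using the actor's class as the item identity lets child Blueprints register as distinct items.
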(event `self.Sphere.OnComponentBeginOverlap`
  (params (OverlappedComponent :type "PrimitiveComponent Object Reference") (OtherActor :type "Actor Object Reference") (OtherComp :type "PrimitiveComponent Object Reference") (OtherBodyIndex :type Integer) (bFromSweep :type Boolean) (SweepResult :type "HitResult Structure (by ref)"))
  (bind _asbp_player (cast `/Game/Blueprints/BP_Player` OtherActor))
  (`/Game/Blueprints/Inventory/BP_MainCryptor.addItem` (`/Game/Blueprints/Core/BP_MainPC.Cryptor` (`/Game/Blueprints/BP_Player.PlayerController` _asbp_player)) (`GameplayStatics.GetObjectClass` self) (`self.count`))
  (`self.K2_DestroyActor`))

(fn `UserConstructionScript`
  (`StaticMeshComponent.SetStaticMesh` (`self.StaticMesh`) (`self.mesh`)))